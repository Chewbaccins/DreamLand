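; BP_Teleport is a box trigger that either moves the player to a linked teleporter or loads another level.
; When TargetLevel is "none", an overlapping third-person character jumps to the TeleportTo box; otherwise any overlap opens the named level.
; A PlayerCanTeleport flag on the game mode gives all teleporters a shared five-second cooldown, preventing bounce-back.
; The flag clears before TeleportTo is validated, so an invalid target leaves teleporting disabled.
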(event `self.Box.OnComponentBeginOverlap`
  (params (OverlappedComponent :type "PrimitiveComponent Object Reference") (OtherActor :type "Actor Object Reference") (OtherComp :type "PrimitiveComponent Object Reference") (OtherBodyIndex :type Integer) (bFromSweep :type Boolean) (SweepResult :type "HitResult Structure (by ref)"))
  (bind _teleportto (`self.TeleportTo`))
  (if (== (`self.TargetLevel`) "none")
    (bind _asbp_third_person_character (cast `/Game/ThirdPerson/Blueprints/BP_ThirdPersonCharacter` OtherActor))
    (bind _asbp_third_person_game_mode (cast `/Game/ThirdPerson/Blueprints/BP_ThirdPersonGameMode` (`GameplayStatics.GetGameMode`)))
    (if (`/Game/ThirdPerson/Blueprints/BP_ThirdPersonGameMode.PlayerCanTeleport` _asbp_third_person_game_mode)
      (`KismetSystemLibrary.Delay` 0.0)
      (set `/Game/ThirdPerson/Blueprints/BP_ThirdPersonGameMode.PlayerCanTeleport` false _asbp_third_person_game_mode)
      (if (`KismetSystemLibrary.IsValid` _teleportto)
        (`SceneComponent.K2_SetWorldLocation` (`Actor.RootComponent` _asbp_third_person_character) (`SceneComponent.K2_GetComponentLocation` (`/Game/BluePrints/BP_Teleport.Box` _teleportto)) false false)
        (`KismetSystemLibrary.Delay` 5.0)
        (set `/Game/ThirdPerson/Blueprints/BP_ThirdPersonGameMode.PlayerCanTeleport` true _asbp_third_person_game_mode)))
    (else
      (`GameplayStatics.OpenLevel` (`self.TargetLevel`)))))

(fn `UserConstructionScript`)